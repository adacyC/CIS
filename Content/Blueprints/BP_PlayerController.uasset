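; Player controller Blueprint that lets a player spawn and despawn their ship through gamepad input.
; On BeginPlay it casts the game mode to BP_CISGameModeBaseMoved and caches the reference.
; The right special gamepad button calls SpawnShip on that game mode and the left calls DespawnShip, each passing the controller itself.
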(event `self.ReceiveBeginPlay`
  (bind _asbp_cisgame_mode_base_moved (cast `/Game/Blueprints/BP_CISGameModeBaseMoved` (`GameplayStatics.GetGameMode`)))
  (set `self.BP_GameMode` _asbp_cisgame_mode_base_moved))

(event `Key|Gamepad_Special_Right`
  (params (Key :type "Key Structure"))
  (:`Pressed`
    (`/Game/Blueprints/BP_CISGameModeBaseMoved.SpawnShip` (`self.BP_GameMode`) self)))

(event `Key|Gamepad_Special_Left`
  (params (Key :type "Key Structure"))
  (:`Pressed`
    (`/Game/Blueprints/BP_CISGameModeBaseMoved.DespawnShip` (`self.BP_GameMode`) self)))

(fn `UserConstructionScript`)