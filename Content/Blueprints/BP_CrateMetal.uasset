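; BP_CrateMetal is a moving metal crate actor that tumbles as it travels and destroys itself on hit.
; BeginPlay rolls random signed spin rates for roll, pitch and yaw.
; Tick sweeps the actor along world negative X by a fixed step per frame, so travel speed depends on frame rate.
; The Box component's local rotation is scaled by delta time, keeping the spin frame-rate independent.
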(event `self.ReceiveBeginPlay`
  (set `self.RandomRoll` (`KismetMathLibrary.RandomFloatInRange` -100.0 100.0))
  (set `self.RandomPitch` (`KismetMathLibrary.RandomFloatInRange` -100.0 100.0))
  (set `self.RandomYaw` (`KismetMathLibrary.RandomFloatInRange` -100.0 100.0)))

(event `self.ReceiveTick`
  (params (DeltaSeconds :type "Float (single-precision)"))
  (bind _box (`self.Box`))
  (set `self.DeltaSeconds` DeltaSeconds)
  (bind _output_get (set `self.CurrentLocation` (`self.K2_GetActorLocation`)))
  (`self.K2_SetActorLocation` (+ _output_get (-5.0 0.0 0.0)) true)
  (`/Engine/EditorBlueprintResources/StandardMacros.IsValid` _box
    (:`Is Valid`
      (`SceneComponent.K2_AddLocalRotation` _box (`KismetMathLibrary.MakeRotator` (* (`self.DeltaSeconds`) (`self.RandomRoll`)) (* (`self.DeltaSeconds`) (`self.RandomPitch`)) (* (`self.DeltaSeconds`) (`self.RandomYaw`))) false false))))

(event `self.ReceiveHit`
  (params (MyComp :type "PrimitiveComponent Object Reference") (Other :type "Actor Object Reference") (OtherComp :type "PrimitiveComponent Object Reference") (bSelfMoved :type Boolean) (HitLocation :type "Vector Structure") (HitNormal :type "Vector Structure") (NormalImpulse :type "Vector Structure") (Hit :type "HitResult Structure (by ref)"))
  (`self.K2_DestroyActor`))

(fn `UserConstructionScript`)