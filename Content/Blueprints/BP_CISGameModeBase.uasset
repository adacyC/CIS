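; BP_CISGameModeBase is a game mode that runs a timed score round and ends it when the countdown reaches zero.
; BeginPlay creates the BPW_HUD widget and sets game-only input, while Tick uses a Delay as a one-second countdown when the timer is enabled.
; SetScore adds to Score and updates HighScore.
; GameOver stops the timer, clears widgets, stores FinalScore in the game instance and opens the GameOver level.
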(event `self.ReceiveBeginPlay`
  (`self.SetScore` 0)
  (bind _returnvalue (`|CreateWidget` "/Game/Blueprints/UserInterface/BPW_HUD.BPW_HUD_C"))
  (bind _output_get (set `self.BP_HUD` _returnvalue))
  (`UserWidget.AddToViewport` _output_get 0)
  (`WidgetBlueprintLibrary.SetInputMode_GameOnly` (`GameplayStatics.GetPlayerController` 0)))

(event `self.ReceiveTick`
  (params (DeltaSeconds :type "Float (single-precision)"))
  (bind _remainingtime (`self.RemainingTime`))
  (`KismetSystemLibrary.Delay` 1.0)
  (if (`self.TimerEnabled`)
    (set `self.RemainingTime` (- _remainingtime 1))
    (if (== 0 _remainingtime)
      (`self.GameOver`))))

(fn `GameOver`
  (set `self.TimerEnabled` false)
  (`WidgetLayoutLibrary.RemoveAllWidgets`)
  (bind _asbp_cisgame_instance (cast `/Game/Blueprints/BP_CISGameInstance` (`GameplayStatics.GetGameInstance`)))
  (set `/Game/Blueprints/BP_CISGameInstance.FinalScore` (`self.Score`) _asbp_cisgame_instance)
  (`GameplayStatics.OpenLevel` "GameOver"))

(fn `SetScore`
  (params (Value :type Integer))
  (set `self.Score` (+ Value (`self.Score`)))
  (if (>= (`self.Score`) (`self.HighScore`))
    (set `self.HighScore` (`self.Score`))))

(fn `UserConstructionScript`)