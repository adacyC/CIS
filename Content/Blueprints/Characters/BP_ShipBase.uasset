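; BP_ShipBase is a player ship with primary and secondary weapons, health, and a game-over on death.
; Held inputs run looping timers that call a shared Fire function, spawning paired primary or single secondary projectiles, with delay checks on each press.
; Hitting a metal crate damages both crate and ship.
; Damage reduces health, and reaching zero calls GameOver on the game mode cached at BeginPlay.
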(event `self.ReceiveBeginPlay`
  (bind _asbp_cisgame_mode_base_moved (cast `/Game/Blueprints/BP_CISGameModeBaseMoved` (`GameplayStatics.GetGameMode`)))
  (set `self.BP_CISGameModeBase` _asbp_cisgame_mode_base_moved)
  (set `self.Health` (`self.MaximumHealth`)))

(event `PrimFire`
  (`self.Fire` (`SceneComponent.K2_GetComponentToWorld` (`self.ProjectileSpawnB`)) "/Game/Blueprints/BP_ProjectileShipBase.BP_ProjectileShipBase_C" :!label _label)
  (`self.Fire` (`SceneComponent.K2_GetComponentToWorld` (`self.ProjectileSpawnT`)) "/Game/Blueprints/BP_ProjectileShipBase.BP_ProjectileShipBase_C")
  (set `self.LastTimeFiredPrimary` (`KismetSystemLibrary.GetGameTimeInSeconds`)))

(event `InputAction|PrimaryFire`
  (params (Key :type "Key Structure"))
  (:`Pressed`
    (if (< (`self.LastTimeFiredPrimary`) (- (`KismetSystemLibrary.GetGameTimeInSeconds`) (`self.FireDelayPrimary`)))
      (`KismetSystemLibrary.K2_SetTimer` null "PrimFire" 0.2 true)
      (goto _label)))
  (:`Released`
    (`KismetSystemLibrary.K2_ClearTimer` null "PrimFire")))

(event `SecFire`
  (`self.Fire` (`SceneComponent.K2_GetComponentToWorld` (`self.ProjectileSpawnC`)) "/Game/Blueprints/BP_ProjectileShipSecondary.BP_ProjectileShipSecondary_C" :!label _label_2)
  (set `self.LastTimeFiredSecondary` (`KismetSystemLibrary.GetGameTimeInSeconds`)))

(event `InputAction|SecondaryFire`
  (params (Key :type "Key Structure"))
  (:`Pressed`
    (if (< (`self.LastTimeFiredSecondary`) (- (`KismetSystemLibrary.GetGameTimeInSeconds`) (`self.FireDelaySecondary`)))
      (`KismetSystemLibrary.K2_SetTimer` null "SecFire" 2.0 true)
      (goto _label_2)))
  (:`Released`
    (`KismetSystemLibrary.K2_ClearTimer` null "SecFire")))

(event `self.ReceiveHit`
  (params (MyComp :type "PrimitiveComponent Object Reference") (Other :type "Actor Object Reference") (OtherComp :type "PrimitiveComponent Object Reference") (bSelfMoved :type Boolean) (HitLocation :type "Vector Structure") (HitNormal :type "Vector Structure") (NormalImpulse :type "Vector Structure") (Hit :type "HitResult Structure (by ref)"))
  (bind _asbp_crate_metal (cast `/Game/Blueprints/BP_CrateMetal` Other))
  (`GameplayStatics.ApplyDamage` _asbp_crate_metal 30.0)
  (`GameplayStatics.ApplyDamage` self 10.0))

(event `self.ReceiveAnyDamage`
  (params (Damage :type "Float (single-precision)") (DamageType :type "DamageType Object Reference") (InstigatedBy :type "Controller Object Reference") (DamageCauser :type "Actor Object Reference"))
  (set `self.Health` (- (`self.Health`) Damage))
  (if (<= (`self.Health`) 0.0)
    (`/Game/Blueprints/BP_CISGameModeBaseMoved.GameOver` (`self.BP_CISGameModeBase`))))

(fn `Fire`
  (params (SpawnTransform :type "Transform Structure") (ProjectileType :type "Actor Class Reference"))
  (locals (ProjectileColour :type "LinearColor Structure" :default (struct :`R` 1.0 :`B` 0.010747)))
  (`|SpawnActorFromClass` ProjectileType SpawnTransform "AlwaysSpawn" "OverrideRootScale" null self))

(fn `UserConstructionScript`)