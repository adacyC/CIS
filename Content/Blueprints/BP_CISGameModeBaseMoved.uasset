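; Game mode for a timed ship game that manages player creation, spawning, score and game over.
; On BeginPlay it gathers PlayerStarts, creates a local player and adds the HUD.
; Spawn and despawn events swap each controller's pawn between large ship and InitPawn, adjusting the spawn index and keeping a shared GameCamera view.
; A delayed Tick counts down to GameOver, which saves the score to the game instance and opens the GameOver level.
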(event `self.ReceiveBeginPlay`
  (bind _numberofplayers (`self.NumberOfPlayers`))
  (bind _outactors (`GameplayStatics.GetAllActorsOfClass` "/Script/Engine.PlayerStart"))
  (set `self.SpawnPoints` _outactors)
  (while (<= _numberofplayers 0)
    (set `self.NumberOfPlayers` (+ _numberofplayers 1))
    (`GameplayStatics.CreatePlayer` -1))
  (`self.SetScore` 0)
  (bind _returnvalue (`|CreateWidget` "/Game/Blueprints/UserInterface/BPW_HUD.BPW_HUD_C"))
  (bind _output_get (set `self.BP_HUD` _returnvalue))
  (`UserWidget.AddToViewport` _output_get 0)
  (`WidgetBlueprintLibrary.SetInputMode_GameOnly` (`GameplayStatics.GetPlayerController` 0)))

(event `self.ReceiveTick`
  (params (DeltaSeconds :type "Float (single-precision)"))
  (bind _remainingtime (`self.RemainingTime`))
  (`KismetSystemLibrary.Delay` 1.0)
  (if (`self.TimerEnabled`)
    (set `self.RemainingTime` (- _remainingtime 1))
    (if (== 0 _remainingtime)
      (`self.GameOver`))))

(event `SpawnShip`
  (params (PlayerController :type "/Game/Blueprints/BP_PlayerController Object Reference"))
  (bind _returnvalue (`Controller.K2_GetPawn` PlayerController))
  (`/Engine/EditorBlueprintResources/StandardMacros.IsValid` _returnvalue
    (:`Is Valid`
      (`self.K2_DestroyActor` _returnvalue)
      (bind _returnvalue_2 (`|SpawnActorFromClass` "/Game/Blueprints/Characters/BP_ShipLarge.BP_ShipLarge_C" (`self.GetSpawnPoint`) "Undefined" "OverrideRootScale" null null))
      (`Controller.Possess` PlayerController _returnvalue_2)
      (`PlayerController.SetViewTargetWithBlend` PlayerController (`self.GameCamera`) 0.0 "VTBlend_Linear" 0.0 false)
      (`/Engine/EditorBlueprintResources/StandardMacros.IncrementInt` (`self.AvailableSpawnPointIndex`)))))

(event `DespawnShip`
  (params (`Player Controller` :type "/Game/Blueprints/BP_PlayerController Object Reference"))
  (bind _returnvalue (`Controller.K2_GetPawn` `Player Controller`))
  (`/Engine/EditorBlueprintResources/StandardMacros.IsValid` _returnvalue
    (:`Is Valid`
      (`self.K2_DestroyActor` _returnvalue)
      (bind _returnvalue_2 (`|SpawnActorFromClass` "/Game/Blueprints/InitPawn.InitPawn_C" (`self.GetSpawnPoint`) "Undefined" "OverrideRootScale" null null))
      (`Controller.Possess` `Player Controller` _returnvalue_2)
      (`PlayerController.SetViewTargetWithBlend` `Player Controller` (`self.GameCamera`) 0.0 "VTBlend_Linear" 0.0 false)
      (`/Engine/EditorBlueprintResources/StandardMacros.DecrementInt` (`self.AvailableSpawnPointIndex`)))))

(fn `GameOver`
  (set `self.TimerEnabled` false)
  (`WidgetLayoutLibrary.RemoveAllWidgets`)
  (bind _asbp_cisgame_instance (cast `/Game/Blueprints/BP_CISGameInstance` (`GameplayStatics.GetGameInstance`)))
  (set `/Game/Blueprints/BP_CISGameInstance.FinalScore` (`self.Score`) _asbp_cisgame_instance)
  (`GameplayStatics.OpenLevel` "GameOver"))

(fn `SetScore`
  (params (Value :type Integer))
  (set `self.Score` (+ Value (`self.Score`)))
  (if (>= (`self.Score`) (`self.HighScore`))
    (set `self.HighScore` (`self.Score`))))

(fn `UserConstructionScript`)