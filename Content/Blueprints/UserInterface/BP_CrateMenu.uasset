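; BP_CrateMenu is an actor that continuously tumbles its static mesh, likely as a decorative crate for the menu.
; On BeginPlay it randomly picks a positive or negative spin rate of equal magnitude for each of roll, pitch and yaw.
; Each Tick it applies those rates, scaled by delta time, as a local rotation to the mesh component when it is valid.
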(event `self.ReceiveBeginPlay`
  (bind _returnvalue (`KismetMathLibrary.RandomBool`))
  (if _returnvalue
    (set `self.RandomRoll` 50)
    (else
      (set `self.RandomRoll` -50)))
  (if _returnvalue
    (set `self.RandomPitch` 50)
    (else
      (set `self.RandomPitch` -50)))
  (if _returnvalue
    (set `self.RandomYaw` 50)
    (else
      (set `self.RandomYaw` -50))))

(event `self.ReceiveTick`
  (params (DeltaSeconds :type "Float (single-precision)"))
  (bind _staticmeshcomponent (`self.StaticMeshComponent`))
  (set `self.DeltaSeconds` DeltaSeconds)
  (`/Engine/EditorBlueprintResources/StandardMacros.IsValid` _staticmeshcomponent
    (:`Is Valid`
      (`SceneComponent.K2_AddLocalRotation` _staticmeshcomponent (`KismetMathLibrary.MakeRotator` (* (`self.RandomRoll`) (`self.DeltaSeconds`)) (* (`self.RandomPitch`) (`self.DeltaSeconds`)) (* (`self.RandomYaw`) (`self.DeltaSeconds`))) false false))))

(fn `UserConstructionScript`)